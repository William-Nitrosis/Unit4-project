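; Arrow projectile Blueprint that deals damage on behalf of the enemy AI that owns it.
; When its Collision component begins overlapping an actor other than itself or an EnemyAi subclass, it prints that actor's name and casts its owner to EnemyAi.
; If the cast succeeds, it applies the owner's AttackDamage to that actor and destroys itself; otherwise the arrow remains.
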(event OnComponentBeginOverlap(Collision)
  (params (OverlappedComponent :type Primitive%20Component%20Object%20Reference) (OtherActor :type Actor%20Object%20Reference) (OtherComp :type Primitive%20Component%20Object%20Reference) (OtherBodyIndex :type Integer) (bFromSweep :type Boolean) (SweepResult :type Hit%20Result%20Structure%20%28by%20ref%29))
  (if (and (not (== OtherActor self)) (not (Utilities|ClassIsChildOf (Utilities|GetClass OtherActor) "/Script/Unit4.enemyAi")))
    (Development|PrintString (Utilities|GetDisplayName OtherActor))
    (bind _asenemy_ai (Utilities|Casting|CastToenemyAi (Components|GetOwner self)))
    (Game|Damage|ApplyDamage OtherActor (Variables|/Script/Unit4.enemyAi|GetAttackDamage _asenemy_ai) 0 0 "/Script/Engine.DamageType")
    (Actor|DestroyActor)))

(event EventBeginPlay)

(fn ConstructionScript)