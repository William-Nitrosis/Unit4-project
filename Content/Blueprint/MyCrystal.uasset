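; MyCrystal is a damageable crystal actor that displays its health on a health bar widget.
; Each tick it casts its Widget component's user widget to the healthbar class and sets the bar's percent from Health against a hard-coded maximum.
; AnyDamage subtracts from Health, and at zero or below clears the Alive flag and destroys the actor.
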(event Game|Damage|EventAnyDamage
  (params (Damage :type Float%20%28single-precision%29) (DamageType :type Damage%20Type%20Object%20Reference) (InstigatedBy :type Controller%20Object%20Reference) (DamageCauser :type Actor%20Object%20Reference))
  (bind _output_get (Variables|Default|Sethealth (- (Variables|Default|Gethealth) Damage)))
  (if (<= _output_get 0.0)
    (Variables|Default|SetAlive false)
    (Actor|DestroyActor)))

(event Collision|EventActorBeginOverlap
  (params (OtherActor :type Actor%20Object%20Reference)))

(event EventBeginPlay)

(event EventTick
  (params (DeltaSeconds :type Float%20%28single-precision%29))
  (bind _ashealthbar (Utilities|Casting|CastTohealthbar (UserInterface|GetUserWidgetObject (Variables|Default|GetWidget))))
  (Progress|SetPercent (Variables|/Game/UI/healthbar.healthbar_C|GethealthBar _ashealthbar) (/ (Variables|Default|Gethealth) 5e+02)))

(fn ConstructionScript)